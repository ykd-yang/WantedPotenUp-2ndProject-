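; BP_BatterTest is a test batter that moves a Box with the mouse cursor and swings on left click.
; BeginPlay gives the Box absolute location and records its depth along the camera's forward axis.
; Each Tick intersects the mouse ray with a camera-facing plane at that depth, moving the Box in world Y and Z with X fixed.
; Clicking plays the hit montage, with SwingEnd blocking another swing until it completes.
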(event EventBeginPlay
  (bind _returnvalue (Game|GetPlayerController 0))
  (bind _box (Variables|Default|GetBox))
  (bind _playercameramanager (Variables|/Script/Engine.PlayerController|GetPlayerCameraManager _returnvalue))
  (Transformation|SetAbsolute _box true false false)
  (Variables|Default|SetCamLoc (Camera|GetCameraLocation _playercameramanager))
  (Variables|Default|SetCamFwd (Math|Vector|GetForwardVector (Camera|GetCameraRotation _playercameramanager)))
  (Variables|Default|SetCubeLoc (Transformation|GetWorldLocation _box))
  (Variables|Default|SetV (- (Variables|Default|GetCubeLoc) (Variables|Default|GetCamLoc)))
  (Variables|Default|SetScreenPlaneDistance (Math|Vector|DotProduct (Variables|Default|GetV) (Variables|Default|GetCamFwd))))

(event EventTick
  (params (DeltaSeconds :type Float%20%28single-precision%29))
  (bind _returnvalue (Game|GetPlayerController 0))
  (bind _returnvalue_2 (Game|GetPlayerCameraManager 0))
  (bind (_worldlocation _worlddirection) (Game|Player|ConvertMouseLocationToWorldSpace _returnvalue))
  ;[0.15 0.15 0.15 0.5] 변수 팅
  (Variables|Default|SetMouseOrigin _worldlocation)
  (Variables|Default|SetMouseDir _worlddirection)
  (Variables|Default|SetMouseRayEnd (+ (* (Variables|Default|GetMouseDir) 1e+05) (Variables|Default|GetMouseOrigin)))
  (Variables|Default|SetCamLoc_Tick (Camera|GetCameraLocation _returnvalue_2))
  (Variables|Default|SetCamFwd_Tick (Math|Vector|GetForwardVector (Camera|GetCameraRotation _returnvalue_2)))
  (Variables|Default|SetPlanePoint (+ (* (Variables|Default|GetCamFwd_Tick) (Variables|Default|GetScreenPlaneDistance)) (Variables|Default|GetCamLoc_Tick)))
  (bind _output_get (Variables|Default|SetPlaneW (* (Math|Vector|DotProduct (Variables|Default|GetPlanePoint) (Variables|Default|GetCamFwd_Tick)) -1.0)))
  (bind _output_get_2 (Variables|Default|SetScreenPlane (Utilities|Struct|MakePlane _output_get (.x (Variables|Default|GetCamFwd_Tick)) (.y (Variables|Default|GetCamFwd_Tick)) (.z (Variables|Default|GetCamFwd_Tick)))))
  (Variables|Default|SetHitPointWorld (.Intersection (Class|KismetMathLibrary|LinePlaneIntersection (Variables|Default|GetMouseOrigin) (Variables|Default|GetMouseRayEnd) _output_get_2)))
  (Transformation|SetWorldLocation (Variables|Default|GetBox) (Math|Vector|MakeVector (.x (Variables|Default|GetCubeLoc)) (.y (Variables|Default|GetHitPointWorld)) (.z (Variables|Default|GetHitPointWorld))) false false))

(event Input|MouseEvents|LeftMouseButton
  (params (Key :type Key%20Structure :default "None"))
  (:Pressed
    (if (not (Variables|Default|GetSwingEnd))
      (Variables|Default|SetSwingEnd true)
      (Animation|Montage|PlayMontage (Variables|Character|GetMesh) "/Game/Asset/Character1/Animation/Batter/Montage/Baseball_Hit_Montage.Baseball_Hit_Montage"
        (:OnCompleted
          (Variables|Default|SetSwingEnd false))))))

(fn ConstructionScript)