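; Batter hit box that follows the mouse cursor on a camera-facing plane and launches BP_TestBall_JW balls it overlaps.
; BeginPlay places the plane in front of the camera; Tick projects the cursor trace onto it to move AimRoot.
; Cube overlap calls NewBattingSystem, which derives velocity from timing, height and side inputs, currently left unconnected.
; An impulse-based restitution/friction model (CheckBatWhere, ApplyHit) remains in uncalled OldVersion.
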(event OnComponentBeginOverlap(Cube)
  (params (OverlappedComponent :type Primitive%20Component%20Object%20Reference) (OtherActor :type Actor%20Object%20Reference) (OtherComp :type Primitive%20Component%20Object%20Reference) (OtherBodyIndex :type Integer) (bFromSweep :type Boolean) (SweepResult :type Hit%20Result%20Structure%20%28by%20ref%29))
  (bind _asbp_test_ball_jw (Utilities|Casting|CastToBP_TestBall_JW OtherActor))
  (CallFunction|NewBattingSystem 0.0 0.0 0.0 _asbp_test_ball_jw))

(event EventBeginPlay
  (bind _returnvalue (Game|GetPlayerController 0))
  (bind _returnvalue_2 (Game|GetPlayerController 0))
  (bind _cursurplaneroot (Variables|Default|GetCurSurPlaneRoot))
  (bind _playercameramanager (Variables|/Script/Engine.PlayerController|GetPlayerCameraManager _returnvalue))
  (bind _returnvalue_3 (Camera|GetCameraRotation _playercameramanager))
  (Variables|/Script/Engine.PlayerController|SetbShowMouseCursor _returnvalue_2 true)
  (Input|SetInputModeGameandUI _returnvalue_2 0 "DoNotLock" true false)
  (Transformation|SetAbsolute (Variables|Default|GetHitBox) true false false)
  (Variables|Default|SetCamLoc (Camera|GetCameraLocation _playercameramanager))
  (Variables|Default|SetCamRot _returnvalue_3)
  (Variables|Default|SetCamFwd (Math|Vector|GetForwardVector _returnvalue_3))
  (Transformation|SetWorldLocation _cursurplaneroot (+ (Variables|Default|GetCamLoc) (* (Variables|Default|GetCamFwd) (Variables|Default|GetDepthOffset))) false false)
  (Transformation|SetWorldRotation _cursurplaneroot (Variables|Default|GetCamRot) false false)
  (Variables|Default|SetPlane (Transformation|GetWorldLocation (Variables|Default|GetCurSurPlaneRoot))))

(event Collision|EventActorBeginOverlap
  (params (OtherActor :type Actor%20Object%20Reference)))

(event EventTick
  (params (DeltaSeconds :type Float%20%28single-precision%29))
  (bind _returnvalue (Game|GetPlayerController 0))
  (bind _camfwd (Variables|Default|GetCamFwd))
  (bind _hitresult (Game|Player|GetHitResultUnderCursorbyChannel _returnvalue "TraceTypeQuery3" true))
  (Variables|Default|SetPlane (Transformation|GetWorldLocation (Variables|Default|GetCurSurPlaneRoot)))
  (bind _output_get (Variables|Default|SetToPlane (- (.impactpoint _hitresult) (Variables|Default|GetPlane))))
  (bind _output_get_2 (Variables|Default|SetDepth (Math|Vector|DotProduct _output_get _camfwd)))
  (bind _output_get_3 (Variables|Default|SetFixed2D (- (.impactpoint _hitresult) (* _output_get_2 _camfwd))))
  (Transformation|SetWorldLocation (Variables|Default|GetAimRoot) _output_get_3 false false))

(fn ConstructionScript)

(fn CheckBatWhere
  (params (Ball :type Actor%20Object%20Reference))
  (bind _cube (Variables|Default|GetCube))
  (bind (_min _max) (Components|StaticMesh|GetLocalBounds _cube))
  (bind _output_get (Variables|Default|SetBallLoc (Transformation|GetActorLocation Ball)))
  (LocalVariables|SetCenterLocal (* (+ _min _max) 0.5))
  (LocalVariables|SetHalfExtent (* (- _max _min) 0.5))
  (bind _output_get_2 (LocalVariables|SetLocal (Math|Transform|InverseTransformLocation (Transformation|GetWorldTransform _cube) _output_get)))
  (LocalVariables|SetLocalCenter (- _output_get_2 (LocalVariables|GetCenterLocal)))
  (Variables|Default|SetContactHeight%20 (* (Math|Float|Clamp(Float) (/ (.z (LocalVariables|GetLocalCenter)) (.z (LocalVariables|GetHalfExtent))) -1.0) -1.0))
  (Variables|Default|SetStrikeSide%20%20%20%20 (Math|Float|Clamp(Float) (/ (.y (LocalVariables|GetLocalCenter)) (.y (LocalVariables|GetHalfExtent))) -1.0))
  (Variables|Default|SetAxIApS (Math|Float|Clamp(Float) (/ (.x (LocalVariables|GetLocalCenter)) (.x (LocalVariables|GetHalfExtent))) -1.0))
  (if (> (Variables|Default|GetContactHeight%20) 0.33)
    (Development|PrintString "상")
    (elif (< (Variables|Default|GetContactHeight%20) -0.33)
      (Development|PrintString "하")
      (else
        (Development|PrintString "중"))))
  (return (Variables|Default|GetContactHeight%20) (Variables|Default|GetStrikeSide%20%20%20%20)))

(fn ApplyHit
  (params (h_BatUpdown :type Float%20%28double-precision%29) (s_BatRightLeft :type Float%20%28double-precision%29) (Timing :type Float%20%28double-precision%29) (ImpactNormalVec :type Vector) (V_ballIn :type Vector))
  (bind _timing_sweet (LocalVariables|GetTiming_Sweet))
  (LocalVariables|SetnormalvecInfunc ImpactNormalVec)
  ;[0.15 0.15 0.15 0.5] 1.개별 벗어난 정도 계싼
  (LocalVariables|SetH_offset (Math|Float|Max(Float) (/ (- (Math|Float|Absolute(Float) h_BatUpdown) (LocalVariables|GetTiming_Sweet)) (- 1.0 (LocalVariables|GetTiming_Sweet))) 0.0))
  ;[0.15 0.15 0.15 0.5] S_offset
  (LocalVariables|SetS_BatOffset (Math|Float|Max(Float) 0.0 (/ (- (Math|Float|Absolute(Float) s_BatRightLeft) (LocalVariables|GetTiming_Sweet)) (- 1.0 (LocalVariables|GetTiming_Sweet)))))
  (LocalVariables|SetT_Offset (Math|Float|Max(Float) (/ (- (Math|Float|Absolute(Float) Timing) _timing_sweet) (- 1.0 _timing_sweet)) 0.0))
  (bind _output_get (LocalVariables|SetA_Offset (|(((a+b)+c)/3) (LocalVariables|GetT_Offset) (LocalVariables|GetH_offset) (LocalVariables|GetS_BatOffset))))
  (LocalVariables|SetE (|(emax+((emin-emax)*a)) (LocalVariables|Gete_Max) (LocalVariables|Gete_Min) _output_get))
  (LocalVariables|SetU (|(ucenter+((uedge-ucenter)*a)) (LocalVariables|GetU_Center) (LocalVariables|GetU_Edge) _output_get))
  (bind _output_get_2 (LocalVariables|SetV_Bat (* (LocalVariables|GetS_Bat) (Math|Vector|Normalize (Math|Vector|CrossProduct ImpactNormalVec "0.000000,0.000000,1.000000")))))
  (LocalVariables|SetV_rel (- V_ballIn _output_get_2))
  (if (< (Math|Vector|DotProduct (LocalVariables|GetV_rel) ImpactNormalVec) 0.0)
    (LocalVariables|SetJ_n (* (* (* (+ (LocalVariables|GetE) 1.0) -1.0) (Math|Vector|DotProduct (LocalVariables|GetV_rel) ImpactNormalVec)) (LocalVariables|GetMass_Ball)))
    (else
      (LocalVariables|SetJ_n 0.0)))
  (LocalVariables|SetV_relT (- (LocalVariables|GetV_rel) (* (Math|Vector|DotProduct (LocalVariables|GetV_rel) ImpactNormalVec) ImpactNormalVec)))
  (LocalVariables|SetJ_t (Math|Float|Min(Float) (* (LocalVariables|GetU) (LocalVariables|GetJ_n)) (* (Math|Vector|VectorLength (LocalVariables|GetV_relT)) (LocalVariables|GetMass_Ball))))
  (LocalVariables|SetJ_total (- (* (LocalVariables|GetJ_n) (LocalVariables|GetnormalvecInfunc)) (* (LocalVariables|GetJ_t) (Math|Vector|Normalize (LocalVariables|GetV_relT)))))
  (return (+ V_ballIn (/ (LocalVariables|GetJ_total) (LocalVariables|GetMass_Ball)))))

(fn OldVersion
  (params (Object :type Object%20Object%20Reference) (Object2 :type Object%20Object%20Reference))
  (Development|PrintString (Utilities|GetDisplayName Object))
  (bind _asbp_test_ball_jw (Utilities|Casting|CastToBP_TestBall_JW Object2))
  (bind (_height _strikeside____) (CallFunction|CheckBatWhere _asbp_test_ball_jw))
  (bind _output_get (Variables|Default|SetHitNormalVector (Math|Vector|Normalize (- (Transformation|GetActorLocation _asbp_test_ball_jw) (.OutPointOnBody (Collision|GetClosestPointonCollision (Variables|Default|GetCube) (Transformation|GetActorLocation _asbp_test_ball_jw) "None"))))))
  (bind _voutspeed (CallFunction|ApplyHit _height _strikeside____ 0.33 _output_get (Variables|/Game/BP/BP_TestBall_JW.BP_TestBall_JW_C|GetVelocity _asbp_test_ball_jw)))
  (Transformation|SetActorRotation _asbp_test_ball_jw "0, 0, 0" true)
  (Variables|/Game/BP/BP_TestBall_JW.BP_TestBall_JW_C|SetIsHitting _asbp_test_ball_jw true)
  (bind _output_get_2 (Variables|/Game/BP/BP_TestBall_JW.BP_TestBall_JW_C|SetVelocity _asbp_test_ball_jw (Math|Vector|MakeVector (Math|Float|Clamp(Float) (.x _voutspeed) -6e+03 -3e+03) (.y _voutspeed) (Math|Float|Clamp(Float) (.z _voutspeed) 2e+03 6e+03))))
  (Development|PrintString (Utilities|String|ToString(Vector) _output_get_2)))

(fn NewBattingSystem
  (params (Timing :type Float%20%28double-precision%29) (HeightBat :type Float%20%28double-precision%29) (SideBat :type Float%20%28double-precision%29) (Ball :type BP%20Test%20Ball%20JW%20Object%20Reference))
  (bind _returnvalue (+ HeightBat 1.0))
  (bind _returnvalue_2 (/ _returnvalue 2.0))
  (bind _returnvalue_3 (Math|Float|Lerp 1.0 0.0 _returnvalue_2))
  (Variables|/Game/BP/BP_TestBall_JW.BP_TestBall_JW_C|SetIsHitting Ball true)
  (Development|PrintString (Utilities|String|ToString(Float) _returnvalue_3))
  ;[0.15 0.15 0.15 0.5] 0으로 초기화
  (Variables|/Game/BP/BP_TestBall_JW.BP_TestBall_JW_C|SetVelocity Ball (* (Math|Vector|Normalize (Math|Vector|MakeVector -1.0 (Math|Float|Lerp 1.0 -1.0 (/ (+ Timing 1.0) 2.0)) _returnvalue_3)) 5e+03 (- 1.0 (Math|Float|Absolute(Float) SideBat)))))