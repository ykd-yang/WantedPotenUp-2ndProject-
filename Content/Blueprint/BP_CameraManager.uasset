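; BP_CameraManager is a camera director that briefly cuts to a ball-following view when the batter hits the ball.
; On BeginPlay it binds to the BP_FinalBatter OnHit event and caches the first player controller.
; A hit points the BallCamera's look-at tracking at the hit ball, then timed delays switch the view target to that camera and back to the CharacterCamera.
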(event Custom|ChangeVIEW
  (params (BaseBallDir :type Float%20%28single-precision%29) (HITBALL :type Ball%20Object%20Reference))
  (bind _ballcamera (Variables|Default|GetBallCamera))
  (Variables|/Script/CinematicCamera.CineCameraActor|SetLookatTrackingSettings _ballcamera (Utilities|Struct|MakeCameraLookatTrackingSettings true true 0.0 (Utilities|ResolveSoftReference HITBALL) "0.000000,0.000000,0.000000" false))
  (Utilities|FlowControl|Delay 1.0)
  (Game|Player|SetViewTargetwithBlend (Variables|Default|GetController) _ballcamera 0.0 "VTBlend_Linear" 0.0 false)
  (Utilities|FlowControl|Delay 2.5)
  (Game|Player|SetViewTargetwithBlend (Variables|Default|GetController) (Variables|Default|GetCharacterCamera) 0.0 "VTBlend_Linear" 0.0 false))

(event EventBeginPlay
  (bind _asbp_final_batter (Utilities|Casting|CastToBP_FinalBatter (Variables|Default|GetBatter)))
  (EventDispatchers|BindEventtoOnHit _asbp_final_batter (delegate Custom|ChangeVIEW))
  (Variables|Default|SetController (Game|GetPlayerController 0)))

(fn ConstructionScript)