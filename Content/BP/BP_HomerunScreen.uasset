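; Breakable home run screen built on a Geometry Collection that cycles random textures on a timer until a ball hits it.
; Each hit adds a cracked-glass decal, sound, electric particles and a briefly shown widget, then calls ChangeToHomeRun.
; The first hit animates screen emission via a dynamic material.
; The second enables gravity and triggers a spawned field actor to shatter it, destroying both shortly after.
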(event Custom|OnFinishDestroy
  (Actor|DestroyActor (stale EventOnBallHit _returnvalue_2))
  (Components|DestroyComponent (Variables|Default|GetGeometryCollection)))

(event Custom|ChangeScreen
  (if (> (Variables|Default|GetHitCnt) 0)
    (Utilities|Time|ClearandInvalidateTimerbyHandle (Variables|Default|GetChangeScreenTimeHandler))
    (else
      (CallFunction|ChangeScreenFunc))))

(event Custom|MakeBlueScreen
  (bind _newtrack_0 (Timeline|Timeline Play)
    (:Update
      (Rendering|Material|SetScalarParameterValue (Variables|Default|GetScreenMat) (Variables|Default|GetEmissionAlpha) _newtrack_0 :!class /Script/Engine.MaterialInstanceDynamic))))

(event EventBeginPlay
  (bind _returnvalue (Rendering|Material|CreateDynamicMaterialInstance (Variables|Default|GetGeometryCollection) 0 "/Game/Effect/M_Screen_Inst.M_Screen_Inst" "None" :!class /Script/Engine.PrimitiveComponent))
  (Variables|Default|SetScreenMat _returnvalue)
  (bind _returnvalue_2 (Utilities|Time|SetTimerbyEvent (delegate Custom|ChangeScreen) 5.0 true))
  (Variables|Default|SetChangeScreenTimeHandler _returnvalue_2))

(event EventOnBallHit
  (params (HitLoctaion :type Vector :default "0, 0, 0"))
  (bind (_x _y _z) (Math|Vector|BreakVector HitLoctaion))
  (bind _widget (Variables|Default|GetWidget))
  (bind _returnvalue (Game|SpawnActorfromClass "/Script/Engine.DecalActor" (Math|Transform|MakeTransform HitLoctaion (Math|Rotator|MakeRotator 0.0 9e+01 0.0) (* (Transformation|GetActorScale3D) 0.1)) "Undefined" "MultiplyWithRoot" 0 0))
  (Rendering|Components|Decal|SetDecalMaterial (Variables|/Script/Engine.DecalActor|GetDecal _returnvalue) "/Game/Effect/M_CrahsedGlassDecal.M_CrahsedGlassDecal")
  (if (Variables|Default|GetIsBreak)
    (Audio|PlaySound2D "/Game/SFX/Destroy/GlassHit.GlassHit" 1.0 1.0 0.0 0 0 false)
    (elif (> (Variables|Default|GetHitCnt) 0)
      (Audio|PlaySound2D "/Game/SFX/Destroy/GlassBreak.GlassBreak" 1.0 1.0 0.0 0 0 false)
      (Physics|SetEnableGravity (Variables|Default|GetGeometryCollection) true)
      (bind _returnvalue_2 (Game|SpawnActorfromClass "/Engine/EditorResources/FieldNodes/FS_MasterField.FS_MasterField_C" (Math|Transform|MakeTransform (+ (* (Math|Vector|Normalize HitLoctaion) 100) (Math|Vector|MakeVector _x _y _z)) "0, 0, 0" "10.000000,20.000000,20.000000") "Undefined" "MultiplyWithRoot" 0 0))
      (Variables|/Engine/EditorResources/FieldNodes/FS_MasterField.FS_MasterField_C|SetActivationType _returnvalue_2 "NewEnumerator4")
      (Default|CETrigger _returnvalue_2)
      (Utilities|Time|SetTimerbyEvent (delegate Custom|OnFinishDestroy) 2.0)
      (Variables|Default|SetIsBreak true)
      (else
        (CallFunction|MakeBlueScreen)
        (Variables|Default|SetHitCnt 1)
        (Audio|PlaySound2D "/Game/SFX/Destroy/GlassHit.GlassHit" 1.0 1.0 0.0 0 0 false))))
  (Effects|SpawnEmitteratLocation "/Game/Asset/Realistic_Starter_VFX_Pack_Vol2/Particles/Destruction/P_Destruction_Electric.P_Destruction_Electric" HitLoctaion "0, 0, 0" "2.000000,2.000000,2.000000")
  (Rendering|SetVisibility _widget true false)
  (Transformation|SetWorldLocation _widget (+ HitLoctaion "0.000000,0.000000,150.000000") false false)
  (Utilities|FlowControl|Delay 2.0)
  (Rendering|SetVisibility (Variables|Default|GetWidget) false false)
  (Class|HomerunEventer|ChangetoHomeRun))

(fn ConstructionScript)

(fn ChangeScreenFunc
  (bind _textures (Variables|Default|GetTextures))
  (bind _outindex (Utilities|Array|Random _textures))
  (if (== _outindex (Variables|Default|GetRandIdx))
    (Variables|Default|SetRandIdx (Math|Integer|%(Integer) (+ (Variables|Default|GetRandIdx) 1) (Utilities|Array|Length (Variables|Default|GetTextures))))
    (else
      (Variables|Default|SetRandIdx _outindex)))
  (Rendering|Material|SetTextureParameterValue (Variables|Default|GetScreenMat) (Variables|Default|GetScreenTexture) (Utilities|Array|Get(acopy) (Variables|Default|GetTextures) (Variables|Default|GetRandIdx))))