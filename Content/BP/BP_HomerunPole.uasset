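; Home run pole actor that plays a celebration when a ball hits it.
; On BeginPlay it resets the scale of its Niagara and particle effects and switches them off.
; OnBallHit moves a widget to the hit location, shows it and activates both effects.
; Timed delays then call ChangeToHomeRun, hide the widget and finally deactivate the effects.
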(event EventOnBallHit
  (params (HitLoctaion :type Vector :default "0, 0, 0"))
  (bind _widget (Variables|Default|GetWidget))
  (Rendering|SetVisibility _widget true false)
  (Transformation|SetWorldLocation _widget HitLoctaion false false)
  (Components|Activation|SetActive (Variables|Default|GetNiagara) true true)
  (Components|Activation|SetActive (Variables|Default|GetParticleSystem1) true true)
  (Utilities|FlowControl|Delay 2.0)
  (Class|HomerunEventer|ChangetoHomeRun)
  (Rendering|SetVisibility (Variables|Default|GetWidget) false false)
  (Utilities|FlowControl|Delay 3.0)
  (Components|Activation|SetActive (Variables|Default|GetNiagara) false true)
  (Components|Activation|SetActive (Variables|Default|GetParticleSystem1) false true))

(event EventBeginPlay
  (Transformation|SetWorldScale3D (Variables|Default|GetParticleSystem1) "1.000000,1.000000,1.000000")
  (Transformation|SetWorldScale3D (Variables|Default|GetNiagara) "1.000000,1.000000,1.000000")
  (Components|Activation|SetActive (Variables|Default|GetNiagara) false true)
  (Components|Activation|SetActive (Variables|Default|GetParticleSystem1) false true))

(fn ConstructionScript)