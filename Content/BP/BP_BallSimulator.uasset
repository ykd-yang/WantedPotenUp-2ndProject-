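; Debug simulator for pitched-ball flight, drawing the trajectory of the "Slider" row from DT_PitchType.
; BeginPlay loads that row's speed, direction and spin into the starting velocity and ball info.
; Tick integrates gravity, Magnus force (spin cross velocity) and AirResistance with a drag-coefficient curve, then draws each step as a debug line.
; Every second it restores the starting velocity and restarts from a slightly randomized start location to vary where pitches land.
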(event EventTick
  (params (DeltaSeconds :type Float%20%28single-precision%29))
  (bind _returnvalue (Math|Random|RandomFloatinRange -1e+01 1e+01))
  (bind _ballinfo (Variables|Default|GetBallInfo))
  (Variables|Default|Settimer (+ DeltaSeconds (Variables|Default|Gettimer)))
  (Variables|Default|SetVelocity (+ (Variables|Default|GetVelocity) (* (Variables|Default|GetGravity) (Utilities|Time|GetWorldDeltaSeconds))))
  (bind _output_get (Variables|Default|SetVelocity (+ (* (* (Math|Vector|CrossProduct (Math|Vector|MakeVector (.rotx _ballinfo) (.roty _ballinfo) (.rotz _ballinfo)) (Variables|Default|GetVelocity)) (Variables|Default|GetMagnusCoeff)) (Utilities|Time|GetWorldDeltaSeconds)) (Variables|Default|GetVelocity))))
  (bind _velocitywithdrag (CallFunction|AirResistance _output_get "/Game/LibraryFunction/Curve_DragCoefficient.Curve_DragCoefficient"))
  (bind _output_get_2 (Variables|Default|SetVelocity _velocitywithdrag))
  (bind _output_get_3 (Variables|Default|SetPrePos (Variables|Default|GetPos)))
  (bind _output_get_4 (Variables|Default|SetPos (+ (Variables|Default|GetPos) (* _output_get_2 (Utilities|Time|GetWorldDeltaSeconds)))))
  (Rendering|Debug|DrawDebugLine :LineStart _output_get_3 :LineEnd _output_get_4 :Duration 1.0 :Thickness 5.0)
  (if (>= (Variables|Default|Gettimer) 1.0)
    (Variables|Default|SetVelocity (Variables|Default|GetStartVel))
    (Variables|Default|SetPos (+ (Variables|Default|GetStartLoc) (Math|Vector|MakeVector _returnvalue _returnvalue _returnvalue)))
    (Variables|Default|Settimer 0.0)))

(event EventBeginPlay
  (Variables|Default|SetPos (Variables|Default|GetStartLoc))
  (bind _returnvalue (Utilities|GetDataTableRow "/Game/Data/DT_PitchType.DT_PitchType" "Slider")
    (:then
      (CallFunction|Init (.balltype _returnvalue) (.speed (.pitch_info _returnvalue)) (.rotx (.pitch_info _returnvalue)) (.roty (.pitch_info _returnvalue)) (.rotz (.pitch_info _returnvalue)) (Math|Vector|Normalize (.dir (.pitch_info _returnvalue)))))))

(fn ConstructionScript)

(fn Init
  (params (BallType :type BallType%20Enum :default "NewEnumerator0") (Ball%20Info%20Speed :type Float%20%28double-precision%29) (Ball%20Info%20Rot%20X :type Float%20%28double-precision%29) (Ball%20Info%20Rot%20Y :type Float%20%28double-precision%29) (Ball%20Info%20Rot%20Z :type Float%20%28double-precision%29) (Ball%20Info%20Dir :type Vector))
  (Variables|Default|SetBallType BallType)
  (Variables|Default|SetBallInfo (Utilities|Struct|MakeBall_Info Ball%20Info%20Speed Ball%20Info%20Rot%20X Ball%20Info%20Rot%20Y Ball%20Info%20Rot%20Z Ball%20Info%20Dir))
  (bind _output_get (Variables|Default|SetVelocity (* Ball%20Info%20Speed Ball%20Info%20Dir)))
  (Variables|Default|SetStartVel _output_get))