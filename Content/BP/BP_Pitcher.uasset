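; BP_Pitcher is a baseball pitcher actor that holds a ball and throws it when its ThrowBall event fires.
; On BeginPlay it spawns BP_TestBall_JW and attaches it to the skeletal mesh's right-hand socket.
; Throwing detaches the ball, initializes it with pitch data from DT_PitchType and clears the Throw flag.
; Despite its name, GetRandomPitchType always reads the ChangeUp row, leaving the random pick unused.
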(event Custom|ThrowBall
  (CallFunction|ThrowBallFunc))

(event EventBeginPlay
  (Variables|Default|SetThrow true)
  (CallFunction|SpawnBall))

(event Collision|EventActorBeginOverlap
  (params (OtherActor :type Actor%20Object%20Reference)))

(event EventTick
  (params (DeltaSeconds :type Float%20%28single-precision%29)))

(fn ConstructionScript)

(fn SpawnBall
  (bind _returnvalue (Game|SpawnActorfromClass "/Game/BP/BP_TestBall_JW.BP_TestBall_JW_C" (Math|Transform|MakeTransform "0, 0, 0" "0, 0, 0" "1.000000,1.000000,1.000000") "Undefined" "MultiplyWithRoot" 0 0))
  (bind _output_get (Variables|Default|SetBall _returnvalue))
  (Transformation|AttachComponentToComponent _output_get (Variables|Default|GetSkeletalMesh) "RightHandSocket" "SnapToTarget" "KeepWorld" "KeepRelative" true))

(fn ThrowBallFunc
  (Transformation|DetachFromActor (Variables|Default|GetBall) "KeepWorld" "KeepWorld" "KeepRelative")
  (bind _pitchdata (CallFunction|GetRandomPitchType))
  (Default|Init (Variables|Default|GetBall) (.balltype _pitchdata) (.speed (.pitch_info _pitchdata)) (.rotx (.pitch_info _pitchdata)) (.roty (.pitch_info _pitchdata)) (.rotz (.pitch_info _pitchdata)) (Math|Vector|Normalize (.dir (.pitch_info _pitchdata))))
  (Variables|Default|SetThrow false))

(fn GetRandomPitchType
  (bind _outrownames (DataTable|GetDataTableRowNames "/Game/Data/DT_PitchType.DT_PitchType"))
  (bind _returnvalue (Utilities|GetDataTableRow "/Game/Data/DT_PitchType.DT_PitchType" "ChangeUp")
    (:then
      (return _returnvalue))))