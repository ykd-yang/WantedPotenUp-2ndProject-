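; BP_HomeRunWall is an overlap trigger that detects when a Ball reaches it, counting as a home run in the baseball game.
; On overlap it tells the baseball game mode's in-game UI to display the home run state, then starts a delayed timer that destroys the ball.
; A DestroyActive flag guards the timer and is never reset here, so only the first overlap schedules a destroy.
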(event Custom|DestroyEvent
  (Actor|DestroyActor (stale Collision|EventActorBeginOverlap _asball)))

(event EventBeginPlay
  (bind _asbp_base_ball_game_mode (Utilities|Casting|CastToBP_BaseBallGameMode (Game|GetGameMode)))
  (Variables|Default|SetBaseBallGameMode _asbp_base_ball_game_mode))

(event Collision|EventActorBeginOverlap
  (params (OtherActor :type Actor%20Object%20Reference))
  (bind _asball (Utilities|Casting|CastToBall OtherActor))
  (Class|InGameUI|DisplayHomerunState (Variables|/Script/HomeRunClashCopy.BaseBallGameMode|GetInGameUI (Variables|Default|GetBaseBallGameMode)) true)
  (if (not (Variables|Default|GetbDestroyActive))
    (Variables|Default|SetbDestroyActive true)
    (Utilities|Time|SetTimerbyEvent (delegate Custom|DestroyEvent) 2.5)))

(event EventTick
  (params (DeltaSeconds :type Float%20%28single-precision%29)))

(fn ConstructionScript)