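; Destructible Blueprint that reacts to a ball hit with a falling Geometry Collection and a popup, apparently for a home run moment.
; On hit it enables gravity, applies a downward velocity-change impulse and shows a widget above the hit location.
; After a short delay it ignores all collision except one custom game channel, hides the widget and calls ChangeToHomeRun.
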(event EventOnBallHit
  (params (HitLoctaion :type Vector :default "0, 0, 0"))
  (bind _geometrycollection (Variables|Default|GetGeometryCollection))
  (bind _widget (Variables|Default|GetWidget))
  (bind _geometrycollection_2 (Variables|Default|GetGeometryCollection))
  (Physics|SetEnableGravity _geometrycollection true)
  (Physics|AddImpulse _geometrycollection "0.000000,0.000000,-10.000000" "None" true)
  (Rendering|SetVisibility _widget true false)
  (Transformation|SetWorldLocation _widget (+ HitLoctaion "0.000000,0.000000,150.000000") false false)
  (Utilities|FlowControl|Delay 2.0)
  (Collision|SetCollisionResponsetoAllChannels _geometrycollection_2 "ECR_Ignore")
  (Collision|SetCollisionResponsetoChannel _geometrycollection_2 "ECC_GameTraceChannel7" "ECR_Block")
  (Rendering|SetVisibility (Variables|Default|GetWidget) false false)
  (Class|HomerunEventer|ChangetoHomeRun))

(fn ConstructionScript)