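; Test ball actor that simulates its own flight with gravity, Magnus spin and air drag.
; Init stores ball type, speed, spin and direction, sets the starting velocity and enables simulation.
; Each tick adds gravity and a simplified Magnus term (spin cross velocity), then applies curve-driven drag through AirResistance.
; The resulting velocity moves the actor directly without sweep, so movement does no collision blocking.
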(event Custom|Move
  (if (Variables|Default|GetIsInit)
    (CallFunction|CalGravity)
    (CallFunction|CalMagnusSimple)
    (bind _velocitywithdrag (CallFunction|AirResistance (Variables|Default|GetVelocity) "/Game/LibraryFunction/Curve_DragCoefficient.Curve_DragCoefficient"))
    (Variables|Default|SetVelocity _velocitywithdrag)
    (CallFunction|UpdateLocate)))

(event EventBeginPlay)

(event Collision|EventActorBeginOverlap
  (params (OtherActor :type Actor%20Object%20Reference)))

(event EventTick
  (params (DeltaSeconds :type Float%20%28single-precision%29))
  (CallFunction|Move))

(fn ConstructionScript)

(fn Init
  (params (ballType :type BallType%20Enum :default "NewEnumerator0") (speed :type Float%20%28double-precision%29) (rotX :type Float%20%28double-precision%29) (rotY :type Float%20%28double-precision%29) (rotZ :type Float%20%28double-precision%29) (Dir :type Vector))
  (Variables|Default|SetBallType ballType)
  (Variables|Default|SetBallInfo (Utilities|Struct|MakeBall_Info speed rotX rotY rotZ Dir))
  (Variables|Default|SetVelocity (* speed Dir))
  (Variables|Default|SetIsInit true))

(fn CalGravity
  (Variables|Default|SetVelocity (+ (Variables|Default|GetVelocity) (* (Variables|Default|GetGravity) (Utilities|Time|GetWorldDeltaSeconds))))
  (return))

(fn CalMagnusSimple
  (bind _ballinfo (Variables|Default|GetBallInfo))
  (Variables|Default|SetVelocity (+ (* (* (Math|Vector|CrossProduct (Math|Vector|MakeVector (.rotx _ballinfo) (.roty _ballinfo) (.rotz _ballinfo)) (Variables|Default|GetVelocity)) (Variables|Default|GetMagnusCoeff)) (Utilities|Time|GetWorldDeltaSeconds)) (Variables|Default|GetVelocity)))
  (return))

(fn UpdateLocate
  (Transformation|SetActorLocation (+ (Transformation|GetActorLocation) (* (Utilities|Time|GetWorldDeltaSeconds) (Variables|Default|GetVelocity))) false false))